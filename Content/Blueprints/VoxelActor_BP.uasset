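; Voxel terrain chunk actor that computes a height noise grid and hosts pickable foliage and ambient effects.
; CalculateNoise layers multi-frequency simplex noise over chunk-offset coordinates, padded past the chunk edge.
; AddInstanceVoxel maps types to instanced plants, butterfly child actors or particles, adding dust to one flower type.
; Overlapping an instance removes it, plays a sound and passes an item to NewPlayerController; ClearExtras wipes all decorations.
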(event `self.AddInstanceVoxel`
  (params (instanceLocation :type "Vector Structure") (type :type Integer))
  (bind _returnvalue (`KismetMathLibrary.RandomFloat`))
  (bind _returnvalue_2 (`KismetMathLibrary.RandomFloat`))
  (bind _particles (`self.Particles`))
  (bind _returnvalue_3 (- (* _returnvalue 100.0) 50.0))
  (bind _returnvalue_4 (`KismetMathLibrary.MakeVector` (.x instanceLocation) (.y instanceLocation) (- (.z instanceLocation) (`KismetMathLibrary.Conv_IntToDouble` (/ (`/Game/Blueprints/NewPlayerController.voxelSize` (cast `/Game/Blueprints/NewPlayerController` (`GameplayStatics.GetPlayerController` 0) :!pure true)) 2)))))
  (bind _returnvalue_5 (`KismetMathLibrary.MakeTransform` (+ _returnvalue_4 (0.0 0.0 800.0)) (`KismetMathLibrary.MakeRotator` 0.0 0.0 (* _returnvalue_2 360.0))))
  (if (>= type 6)
    (switch `int` type
      (:`6`
        (`InstancedStaticMeshComponent.AddInstance` (`self.InstancedMushroom`) (`KismetMathLibrary.MakeTransform` (+ _returnvalue_4 (`KismetMathLibrary.MakeVector` _returnvalue_3 _returnvalue_3)) (struct) (`KismetMathLibrary.Conv_DoubleToVector` (+ (* _returnvalue 0.4) 0.8)))))
      (:`7`
        (bind _returnvalue_6 (`AddComponent|NODE_AddChildActorComponent-0` :`RelativeTransform` (`KismetMathLibrary.MakeTransform` (+ _returnvalue_4 (`KismetMathLibrary.MakeVector` 0.0 0.0 (+ (* _returnvalue_2 200.0) 50.0))) (struct) (`KismetMathLibrary.Conv_DoubleToVector` (+ (`KismetMathLibrary.RandomFloat`) 2.0)))))
        (`KismetArrayLibrary.Array_Add` (`self.butterflies`) _returnvalue_6))
      (:`8`
        (if (`KismetMathLibrary.RandomBool`)
          (bind _returnvalue_7 (`AddComponent|NODE_AddParticleSystemComponent-1` :`bManualAttachment` true :`RelativeTransform` _returnvalue_5))
          (`KismetArrayLibrary.Array_Add` _particles _returnvalue_7)
          (else
            (bind _returnvalue_8 (`AddComponent|NODE_AddParticleSystemComponent-0` :`RelativeTransform` _returnvalue_5))
            (`KismetArrayLibrary.Array_Add` _particles _returnvalue_8))))
      (:`9`
        (bind _returnvalue_9 (`AddComponent|NODE_AddParticleSystemComponent-2` :`RelativeTransform` (`KismetMathLibrary.Conv_VectorToTransform` (+ _returnvalue_4 (0.0 0.0 200.0)))))
        (`KismetArrayLibrary.Array_Add` _particles _returnvalue_9)))
    (else
      (`InstancedStaticMeshComponent.AddInstance` (select `int` type :`0` (`self.InstancedGrass`) :`1` (`self.InstancedFlower1`) :`2` (`self.InstancedFlower2`) :`3` (`self.InstancedFlower3`) :`4` (`self.InstancedFlower4`) :`5` (`self.InstancedSapling`)) (`KismetMathLibrary.Conv_VectorToTransform` _returnvalue_4))
      (`self.spawnDust` _returnvalue_4 type))))

(event `self.InstancedGrass.OnComponentBeginOverlap`
  (params (OverlappedComponent :type "PrimitiveComponent Object Reference") (OtherActor :type "Actor Object Reference") (OtherComp :type "PrimitiveComponent Object Reference") (OtherBodyIndex :type Integer) (bFromSweep :type Boolean) (SweepResult :type "HitResult Structure (by ref)"))
  (`self.instancePick` 0 SweepResult))

(event `self.InstancedFlower1.OnComponentBeginOverlap`
  (params (OverlappedComponent :type "PrimitiveComponent Object Reference") (OtherActor :type "Actor Object Reference") (OtherComp :type "PrimitiveComponent Object Reference") (OtherBodyIndex :type Integer) (bFromSweep :type Boolean) (SweepResult :type "HitResult Structure (by ref)"))
  (`self.instancePick` 1 SweepResult))

(event `self.InstancedFlower2.OnComponentBeginOverlap`
  (params (OverlappedComponent :type "PrimitiveComponent Object Reference") (OtherActor :type "Actor Object Reference") (OtherComp :type "PrimitiveComponent Object Reference") (OtherBodyIndex :type Integer) (bFromSweep :type Boolean) (SweepResult :type "HitResult Structure (by ref)"))
  (bind (_bblockinghit _binitialoverlap _time _distance _location _impactpoint _normal _impactnormal _physmat _hitactor _hitcomponent _hitbonename _hititem) (`GameplayStatics.BreakHitResult` SweepResult))
  (bind _dusts (`self.dusts`))
  (`self.instancePick` 2 SweepResult)
  (`ActorComponent.K2_DestroyComponent` (`|GetArrayItem` _dusts _hititem))
  (`KismetArrayLibrary.Array_Remove` _dusts _hititem))

(event `self.InstancedFlower3.OnComponentBeginOverlap`
  (params (OverlappedComponent :type "PrimitiveComponent Object Reference") (OtherActor :type "Actor Object Reference") (OtherComp :type "PrimitiveComponent Object Reference") (OtherBodyIndex :type Integer) (bFromSweep :type Boolean) (SweepResult :type "HitResult Structure (by ref)"))
  (`self.instancePick` 3 SweepResult))

(event `self.InstancedFlower4.OnComponentBeginOverlap`
  (params (OverlappedComponent :type "PrimitiveComponent Object Reference") (OtherActor :type "Actor Object Reference") (OtherComp :type "PrimitiveComponent Object Reference") (OtherBodyIndex :type Integer) (bFromSweep :type Boolean) (SweepResult :type "HitResult Structure (by ref)"))
  (`self.instancePick` 4 SweepResult))

(event `self.InstancedMushroom.OnComponentBeginOverlap`
  (params (OverlappedComponent :type "PrimitiveComponent Object Reference") (OtherActor :type "Actor Object Reference") (OtherComp :type "PrimitiveComponent Object Reference") (OtherBodyIndex :type Integer) (bFromSweep :type Boolean) (SweepResult :type "HitResult Structure (by ref)"))
  (`self.instancePick` 5 SweepResult))

(event `self.InstancedSapling.OnComponentBeginOverlap`
  (params (OverlappedComponent :type "PrimitiveComponent Object Reference") (OtherActor :type "Actor Object Reference") (OtherComp :type "PrimitiveComponent Object Reference") (OtherBodyIndex :type Integer) (bFromSweep :type Boolean) (SweepResult :type "HitResult Structure (by ref)"))
  (`self.instancePick` 6 SweepResult))

(fn `calculateNoise`
  (locals (xLoc :type Integer) (yLoc :type Integer) (noise :type "Array of Integer"))
  (bind _chunklineelements (`self.chunkLineElements`))
  (for _index (range -1 (+ _chunklineelements 1))
    (set `local.yLoc` _index)
    (for _index_2 (range -1 (+ _chunklineelements 1))
      (set `local.xLoc` _index_2)
      (bind _returnvalue (`SimplexNoiseLibrary.SimplexNoise2D` (* (+ (`local.xLoc`) (* (`self.chunkXindex`) (`self.chunkLineElements`))) 0.01) (* (+ (`local.yLoc`) (* (`self.chunkYindex`) (`self.chunkLineElements`))) 0.01)))
      (bind _returnvalue_2 (`SimplexNoiseLibrary.SimplexNoise2D` (* (+ (`local.xLoc`) (* (`self.chunkXindex`) (`self.chunkLineElements`))) 0.01) (* (+ (`local.yLoc`) (* (`self.chunkYindex`) (`self.chunkLineElements`))) 0.01)))
      (bind _returnvalue_3 (`SimplexNoiseLibrary.SimplexNoise2D` (* (+ (`local.xLoc`) (* (`self.chunkXindex`) (`self.chunkLineElements`))) 0.004) (* (+ (`local.yLoc`) (* (`self.chunkYindex`) (`self.chunkLineElements`))) 0.004)))
      (bind _returnvalue_4 (`SimplexNoiseLibrary.SimplexNoise2D` (* (+ (`local.xLoc`) (* (`self.chunkXindex`) (`self.chunkLineElements`))) 0.05) (* (+ (`local.yLoc`) (* (`self.chunkYindex`) (`self.chunkLineElements`))) 0.05)))
      (`KismetArrayLibrary.Array_Add` (`local.noise`) (`KismetMathLibrary.FFloor` (+ (* _returnvalue 4.0) (* _returnvalue_2 8.0) (* _returnvalue_3 16.0) (`KismetMathLibrary.FClamp` (* _returnvalue_4 4.0) 0.0 5.0))))))
  (return))

(fn `clearExtras`
  (`InstancedStaticMeshComponent.ClearInstances` (`self.InstancedFlower1`))
  (`InstancedStaticMeshComponent.ClearInstances` (`self.InstancedFlower2`))
  (`InstancedStaticMeshComponent.ClearInstances` (`self.InstancedFlower3`))
  (`InstancedStaticMeshComponent.ClearInstances` (`self.InstancedFlower4`))
  (`InstancedStaticMeshComponent.ClearInstances` (`self.InstancedMushroom`))
  (`InstancedStaticMeshComponent.ClearInstances` (`self.InstancedSapling`))
  (`InstancedStaticMeshComponent.ClearInstances` (`self.InstancedGrass`))
  (for _array_element (`self.butterflies`)
    (`ActorComponent.K2_DestroyComponent` _array_element))
  (for _array_element_2 (`self.Particles`)
    (`ActorComponent.K2_DestroyComponent` _array_element_2))
  (for _array_element_3 (`self.dusts`)
    (`ActorComponent.K2_DestroyComponent` _array_element_3))
  (`KismetArrayLibrary.Array_Clear` (`self.butterflies`))
  (`KismetArrayLibrary.Array_Clear` (`self.Particles`))
  (`KismetArrayLibrary.Array_Clear` (`self.dusts`)))

(fn `instancePick`
  (params (itemID :type Integer) (hitElement :type "HitResult Structure"))
  (bind (_bblockinghit _binitialoverlap _time _distance _location _impactpoint _normal _impactnormal _physmat _hitactor _hitcomponent _hitbonename _hititem) (`GameplayStatics.BreakHitResult` hitElement))
  (bind _asinstanced_static_mesh_component (cast `InstancedStaticMeshComponent` _hitcomponent))
  (bind _returnvalue (`InstancedStaticMeshComponent.RemoveInstance` _asinstanced_static_mesh_component _hititem))
  (if _returnvalue
    (`GameplayStatics.PlaySound2D` "/Game/Audio/instancePick_Cue.instancePick_Cue" 1.0 1.0 0.0 null null)
    (`/Game/Blueprints/NewPlayerController.pickItem` (cast `/Game/Blueprints/NewPlayerController` (`GameplayStatics.GetPlayerController` 0) :!pure true) (+ itemID 9))))

(fn `reinitializeInstanceStaticMeshComponent417`
  (params (Reini :type "InstancedStaticMeshComponent Object Reference"))
  (locals (Instances :type "Array of Transform Structure"))
  (bind _instances (`local.Instances`))
  (for _index (range (`InstancedStaticMeshComponent.GetInstanceCount` Reini))
    (`KismetArrayLibrary.Array_Add` _instances (`InstancedStaticMeshComponent.GetInstanceTransform` Reini _index false)))
  (`InstancedStaticMeshComponent.ClearInstances` Reini)
  (for _array_element _instances
    (`InstancedStaticMeshComponent.AddInstance` Reini _array_element)))

(fn `spawnDust`
  (params (location :type "Vector Structure") (type :type Integer))
  (if (== type 2)
    (bind _returnvalue (`AddComponent|NODE_AddParticleSystemComponent-3` :`RelativeTransform` (`KismetMathLibrary.Conv_VectorToTransform` location)))
    (`KismetArrayLibrary.Array_Add` (`self.dusts`) _returnvalue)))

(fn `UserConstructionScript`)