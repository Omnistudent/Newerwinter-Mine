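; MenuPlayerController is a player controller, named for the menu, that applies saved graphics settings on BeginPlay.
; It loads the SettingsBP save from the "Settings" slot, first creating and saving a default one if none exists.
; Each Graphics value is appended to the GraphicCommands entry at the same index and run as a console command, followed by a screen percentage command built from the saved Resolution.
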(event `self.ReceiveBeginPlay`
  (`self.loadGraphicSettings`))

(fn `loadGraphicSettings`
  (bind _settings (`self.Settings`))
  (bind _returnvalue (`GameplayStatics.DoesSaveGameExist` "Settings"))
  (if (not _returnvalue)
    (bind _returnvalue_2 (`GameplayStatics.CreateSaveGameObject` "/Game/UMG/SettingsBP.SettingsBP_C")) ; default
    (bind _assettings_bp (cast `/Game/UMG/SettingsBP` _returnvalue_2))
    (`GameplayStatics.SaveGameToSlot` _assettings_bp "Settings"))
  (bind _returnvalue_3 (`GameplayStatics.LoadGameFromSlot` "Settings"))
  (bind _assettings_bp_2 (cast `/Game/UMG/SettingsBP` _returnvalue_3))
  (set `self.Settings` _assettings_bp_2)
  (for (_array_element _array_index) (`/Game/UMG/SettingsBP.Graphics` _settings)
    (`KismetSystemLibrary.ExecuteConsoleCommand` (`KismetStringLibrary.Concat_StrStr` (`|GetArrayItem` (`self.GraphicCommands`) _array_index) (`KismetStringLibrary.Conv_IntToString` _array_element)) null))
  (`KismetSystemLibrary.ExecuteConsoleCommand` (`KismetStringLibrary.Concat_StrStr` "r.ScreenPercentage " (`KismetStringLibrary.Conv_IntToString` (`/Game/UMG/SettingsBP.Resolution` _settings))) null))

(fn `UserConstructionScript`)